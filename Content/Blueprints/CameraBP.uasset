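; Camera Blueprint that pans its CameraRotator component back and forth between two yaw limits.
; The construction script sets the starting pose from HorizontalRotation, with VerticalAngle applied as roll and pitch zeroed.
; Tick steps the yaw by RotationSpeed, preserving roll and pitch, and flips MovingRight once a limit is passed.
; The step is not scaled by delta time, so sweep speed depends on frame rate.
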(event EventTick
  (params (DeltaSeconds :type Float%20%28single-precision%29))
  (bind _camerarotator (Variables|Default|GetCameraRotator))
  (bind _relativerotation (Variables|/Script/Engine.SceneComponent|GetRelativeRotation _camerarotator))
  (if (Variables|Default|GetMovingRight)
    (if (> (Variables|Default|GethorizontalRotation) (Variables|Default|GetMaxPosRotation))
      (Variables|Default|SetMovingRight false)
      (else
        (Variables|Default|SethorizontalRotation (+ (Variables|Default|GethorizontalRotation) (Variables|Default|GetRotationSpeed)))
        (Transformation|SetRelativeRotation _camerarotator (Math|Rotator|MakeRotator (.roll _relativerotation) (.pitch _relativerotation) (Variables|Default|GethorizontalRotation)) false false :!label _label)))
    (elif (< (Variables|Default|GethorizontalRotation) (Variables|Default|GetMaxNegRotation))
      (Variables|Default|SetMovingRight true)
      (else
        (Variables|Default|SethorizontalRotation (- (Variables|Default|GethorizontalRotation) (Variables|Default|GetRotationSpeed)))
        (goto _label)))))

(fn ConstructionScript
  (Transformation|SetRelativeRotation (Variables|Default|GetCameraRotator) (Math|Rotator|MakeRotator (Variables|Default|GetVerticalAngle) 0.0 (Variables|Default|GethorizontalRotation)) false false))