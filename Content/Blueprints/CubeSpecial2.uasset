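; CubeSpecial2 is an interactable actor that toggles the visibility of a DirectionalLight while something overlaps it.
; Any actor overlap enables input from player controller 0 and opens a gate; ending the overlap closes the gate but never disables input.
; With the gate open, pressing E runs a FlipFlop that alternately shows and hides the light, printing "Hello" each time.
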(event EventBeginPlay)

(event EventTick
  (params (DeltaSeconds :type Float%20%28single-precision%29)))

(event Collision|EventActorBeginOverlap
  (params (OtherActor :type Actor%20Object%20Reference))
  (Input|EnableInput (Game|GetPlayerController 0))
  (Utilities|FlowControl|Gate true) ; enters at Open
)

(event Collision|EventActorEndOverlap
  (params (OtherActor :type Actor%20Object%20Reference))
  (Utilities|FlowControl|Gate true) ; enters at Close
)

(event Input|KeyboardEvents|E
  (params (Key :type Key%20Structure :default "AnyKey"))
  (:Pressed
    (Utilities|FlowControl|Gate true
      (:Exit
        (Utilities|FlowControl|FlipFlop
          (:A
            (Rendering|SetVisibility (Variables|Default|GetDirectionalLight) true false)
            (Development|PrintString "Hello"))
          (:B
            (Rendering|SetVisibility (Variables|Default|GetDirectionalLight) false false)
            (Development|PrintString "Hello")))))))

(fn ConstructionScript)