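; Masher hazard that shuttles back and forth along Y and restarts the level shortly after touching the player.
; Start picks the first direction from Flipped, then two delay-stepped custom loops alternate, nudging the actor by fixed steps.
; ShouldStop runs after each stroke, halting only at the starting end when On is false.
; Two collision boxes detect the player; the first also calls Emancipate on CubeSpecial actors.
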(event OnComponentBeginOverlap(CollisionBox)
  (params (OverlappedComponent :type Primitive%20Component%20Object%20Reference) (OtherActor :type Actor%20Object%20Reference) (OtherComp :type Primitive%20Component%20Object%20Reference) (OtherBodyIndex :type Integer) (bFromSweep :type Boolean) (SweepResult :type Hit%20Result%20Structure%20%28by%20ref%29))
  ;[1 1 1] Hit Player
  (if (== OtherActor (Game|GetPlayerCharacter 0))
    (Utilities|FlowControl|Delay 0.6)
    (bind _returnvalue (Game|GetCurrentLevelName true))
    (Game|OpenLevel(byName) (Utilities|String|StringToName _returnvalue))
    (else
      (bind _ascube_special (Utilities|Casting|CastToCubeSpecial OtherActor))
      (Default|Emancipate _ascube_special))))

(event OnComponentBeginOverlap(CollisionBox2)
  (params (OverlappedComponent :type Primitive%20Component%20Object%20Reference) (OtherActor :type Actor%20Object%20Reference) (OtherComp :type Primitive%20Component%20Object%20Reference) (OtherBodyIndex :type Integer) (bFromSweep :type Boolean) (SweepResult :type Hit%20Result%20Structure%20%28by%20ref%29))
  ;[1 1 1] Hit Player
  (if (== OtherActor (Game|GetPlayerCharacter 0))
    (Utilities|FlowControl|Delay 0.6)
    (bind _returnvalue (Game|GetCurrentLevelName true))
    (Game|OpenLevel(byName) (Utilities|String|StringToName _returnvalue))))

(event Custom|Start
  ;[1 1 1] Movement
  (if (Variables|Default|GetFlipped?) ; Decide which way to move first
    (Utilities|ModifiedforLoop 0 45 :!label _label ; Move Backwards
      (:LoopBody
        (Transformation|SetActorRelativeLocation (+ (Transformation|GetActorLocation) "0,-10.000000, 0"))
        (Utilities|FlowControl|Delay 1e-06)
        (goto _label Next%20Step%20In))
      (:Completed
        (CallFunction|ShouldStop? "Backwards")
        (if (not (Variables|Default|GetStopping))
          (Utilities|ModifiedforLoop 0 45 :!label _label_2 ; Move Forwards
            (:LoopBody
              (Transformation|SetActorRelativeLocation (+ (Transformation|GetActorLocation) "0,10.000000, 0"))
              (Utilities|FlowControl|Delay 1e-06)
              (goto _label_2 Next%20Step%20In))
            (:Completed
              (CallFunction|ShouldStop? "Forwards")
              (if (not (Variables|Default|GetStopping))
                (goto _label)))))))
    (else
      (goto _label_2))))

(event Custom|ShouldStop?
  (params (Direction :type String))
  ;[1 1 1] Decide whether to stop
  (Variables|Default|SetStopping false)
  (if (not (Variables|Default|GetOn?))
    (if (or (and (Variables|Default|GetFlipped?) (Utilities|Enum|Equal(Enum) "Forwards" Direction)) (and (not (Variables|Default|GetFlipped?)) (Utilities|Enum|Equal(Enum) "Backwards" Direction)))
      (Variables|Default|SetStopping true)
      (Variables|Default|SetOn? false))))

(fn ConstructionScript)