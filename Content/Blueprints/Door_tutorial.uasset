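; Tutorial double-door Blueprint that moves two door components open when something overlaps its trigger volume.
; The overlap plays a timeline whose Driver track is the alpha for lerping each door's relative location between its own start and end vectors.
; The overlapping actor is not filtered, and no end-overlap or reverse logic closes the doors.
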(event OnComponentBeginOverlap(TriggerVolume)
  (params (OverlappedComponent :type Primitive%20Component%20Object%20Reference) (OtherActor :type Actor%20Object%20Reference) (OtherComp :type Primitive%20Component%20Object%20Reference) (OtherBodyIndex :type Integer) (bFromSweep :type Boolean) (SweepResult :type Hit%20Result%20Structure%20%28by%20ref%29))
  (bind _driver (Timeline|Timeline%20-%20Door%20Driver Play)
    (:Update
      (Transformation|SetRelativeLocation (Variables|Default|GetDoor) (Math|Vector|Lerp(Vector) (Variables|DoorSetup|GetDoorStart) (Variables|DoorSetup|GetDoorEnd) _driver) false false)
      (Transformation|SetRelativeLocation (Variables|Default|GetDoor2) (Math|Vector|Lerp(Vector) (Variables|DoorSetup|GetDoor2Start) (Variables|DoorSetup|GetDoor2End) _driver) false false))))

(fn ConstructionScript)