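; OpeningFloor is an actor whose two cube pieces move when play begins, likely forming a floor that opens.
; On BeginPlay a single timeline plays and drives both cubes through one shared alpha track.
; Each update linearly interpolates each cube's relative location between its own start and end vector variables.
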(event EventBeginPlay
  (bind _newtrack_1 (Timeline|Timeline_0 Play)
    (:Update
      (Utilities|FlowControl|Sequence
        (:then_0
          (Transformation|SetRelativeLocationAndRotation (Variables|Default|GetCube) (Math|Vector|Lerp(Vector) (Variables|Default|GetCube1Start) (Variables|Default|GetCube1End) _newtrack_1) "0, 0, 0" false false))
        (:then_1
          (Transformation|SetRelativeLocationAndRotation (Variables|Default|GetCube2) (Math|Vector|Lerp(Vector) (Variables|Default|GetCube2Start) (Variables|Default|GetCube2End) _newtrack_1) "0, 0, 0" false false))))))

(fn ConstructionScript)