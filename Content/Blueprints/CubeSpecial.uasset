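; CubeSpecial is a physics cube that rewinds through its recorded motion while the player holds the right button, and can be dissolved.
; Tick records world transform and velocities, packing linear and angular velocity into one Transform's location and scale, then pops both histories to rewind.
; Emancipate applies a fire material, disables gravity, slows the cube, then spins and shrinks it through a delayed loop macro before destroying it.
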(event Custom|Emancipate
  (bind _staticmesh (Variables|Default|GetStaticMesh))
  (Variables|Default|SetisDissolving true)
  (Rendering|Material|SetMaterial _staticmesh 0 "/Game/StarterContent/Textures/T_Fire_Tiled_Mat.T_Fire_Tiled_Mat")
  (Physics|SetEnableGravity _staticmesh false)
  (bind _returnvalue (Physics|GetPhysicsLinearVelocity _staticmesh "None"))
  (Physics|SetPhysicsLinearVelocity _staticmesh (/ _returnvalue 100) false "None")
  (Utilities|ModifiedWhileLoop (Math|Vector|NotEqual(Vector) (Variables|Default|GetScale) "0, 0, 0" 0.001) :!label _label
    (:Loop%20Body
      (bind _output_get (Variables|Default|SetScale (- (Variables|Default|GetScale) 0.01)))
      (Transformation|SetActorScale3D _output_get)
      (Transformation|AddWorldRotation (Variables|Default|GetStaticMesh) "0.000000,6.000000,0.000000" false false)
      (Utilities|FlowControl|Delay 0.01)
      (goto _label Next%20Step%20In))
    (:Completed
      (Actor|DestroyActor))))

(event EventBeginPlay
  (bind _asfirst_person_character_1 (Utilities|Casting|CastToFirstPersonCharacter1 (Game|GetPlayerCharacter 0)))
  (Variables|Default|SetCharacter%20Reference _asfirst_person_character_1))

(event EventTick
  (params (DeltaSeconds :type Float%20%28single-precision%29))
  (bind _velocity (Variables|Default|GetVelocity))
  (bind _staticmesh (Variables|Default|GetStaticMesh))
  (bind _staticmesh_2 (Variables|Default|GetStaticMesh))
  (bind _character_reference (Variables|Default|GetCharacter%20Reference))
  (bind _transform (Variables|Default|GetTransform))
  (bind _returnvalue (Utilities|Array|LastIndex _transform))
  (bind _returnvalue_2 (Utilities|Array|LastIndex _velocity))
  (bind _rightbuttonpressed (Variables|/Game/FirstPersonBP/Blueprints/FirstPersonCharacter1.FirstPersonCharacter1_C|GetRightButtonPressed _character_reference))
  (bind _item (Utilities|Array|Get(acopy) _velocity _returnvalue_2))
  (bind (_location _rotation _scale) (Math|Transform|BreakTransform _item))
  (Utilities|FlowControl|Sequence
    (:then_0
      (if _rightbuttonpressed
        (Transformation|SetWorldTransform _staticmesh (Utilities|Array|Get(acopy) _transform _returnvalue) false false)
        (if (> _returnvalue 0)
          (Utilities|Array|RemoveIndex _transform _returnvalue))
        (else
          (Utilities|Array|Add _transform (Transformation|GetWorldTransform _staticmesh)))))
    (:then_1
      (if _rightbuttonpressed
        (Physics|SetPhysicsLinearVelocity _staticmesh _location false "None")
        (Class|PrimitiveComponent|SetPhysicsAngularVelocity _staticmesh _scale false "None")
        (if (> _returnvalue_2 0)
          (Utilities|Array|RemoveIndex _velocity _returnvalue_2))
        (else
          (bind _returnvalue_3 (Physics|GetPhysicsLinearVelocity _staticmesh_2 "None"))
          (bind _returnvalue_4 (Class|PrimitiveComponent|GetPhysicsAngularVelocity _staticmesh_2 "None"))
          (Utilities|Array|Add _velocity (Math|Transform|MakeTransform _returnvalue_3 "0.000000, 0, 0" _returnvalue_4)))))))

(fn ConstructionScript)