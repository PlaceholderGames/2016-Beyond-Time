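; SwitchActor is an interactable switch that responds to the E key while something overlaps it, apparently meant to toggle a CableCart.
; Begin overlap enables player 0's input and opens a Gate, and end overlap closes the Gate.
; Presses pass into a FlipFlop that prints a debug string and clears the CableCart reference on both branches.
; Only branch A then sets Toggle, on that empty reference, and the node setting it false is unwired.
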(event EventBeginPlay)

(event EventTick
  (params (DeltaSeconds :type Float%20%28single-precision%29)))

(event Collision|EventActorBeginOverlap
  (params (OtherActor :type Actor%20Object%20Reference))
  (Input|EnableInput (Game|GetPlayerController 0))
  (Utilities|FlowControl|Gate true) ; enters at Open
)

(event Collision|EventActorEndOverlap
  (params (OtherActor :type Actor%20Object%20Reference))
  (Utilities|FlowControl|Gate true) ; enters at Close
)

(event Input|KeyboardEvents|E
  (params (Key :type Key%20Structure :default "AnyKey"))
  (:Pressed
    (Utilities|FlowControl|Gate true
      (:Exit
        (Utilities|FlowControl|FlipFlop
          (:A
            (Development|PrintString "Hello")
            (bind _output_get (Variables|Default|SetCable%20Cart 0))
            (Variables|/Game/StaticMesh/cablecartActor.cablecartActor_C|SetToggle _output_get true))
          (:B
            (Development|PrintString "Hello")
            (bind _output_get_2 (Variables|Default|SetCable%20Cart 0))))))))

(fn ConstructionScript)