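; SlidingPlatform is an actor Blueprint for a platform that makes one scripted slide and then removes itself.
; On BeginPlay it caches its start location, waits for a configurable delay, then plays MovementTimeline.
; The timeline offsets the location from that start and sets absolute pitch with zero roll and yaw, without sweeping.
; When the timeline finishes, the actor is destroyed.
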(event EventBeginPlay
  (Variables|Default|SetStartPos (Transformation|GetActorLocation))
  (Utilities|FlowControl|Delay (Variables|Default|GetDelay))
  (bind (_direction _rotation _translation) (Timeline|Movement%20Timeline Play)
    (:Update
      (Transformation|SetActorLocation (+ _translation (Variables|Default|GetStartPos)) false false)
      (Transformation|SetActorRotation (Math|Rotator|MakeRotator 0.0 _rotation 0.0)))
    (:Finished
      (Actor|DestroyActor))))

(fn ConstructionScript)