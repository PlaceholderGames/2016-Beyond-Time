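; TrippyTrigger is a one-shot trigger actor that makes a wall appear when the player character overlaps it.
; BeginPlay builds the spawn transform from the Location, Rotation and Scale variables.
; The first player overlap spawns the Wall class at that transform, applies the Material variable to its Cube and clears the Untriggered flag to block repeats.
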(event Collision|EventActorBeginOverlap
  (params (OtherActor :type Actor%20Object%20Reference))
  (if (and (== OtherActor (Game|GetPlayerCharacter 0)) (Variables|Default|GetUntriggered?))
    (bind _returnvalue (Game|SpawnActorfromClass "/Game/Blueprints/TrippyStuff/SpawnObjects/Wall.Wall_C" (Variables|Default|GetTransform) "Undefined" 0 0))
    (Rendering|Material|SetMaterial (Variables|/Game/Blueprints/TrippyStuff/SpawnObjects/Wall.Wall_C|GetCube _returnvalue) 0 (Variables|Default|GetMaterial))
    (Variables|Default|SetUntriggered? false)))

(event EventBeginPlay
  (Variables|Default|SetTransform (Math|Transform|MakeTransform (Variables|Default|GetLocation) (Variables|Default|GetRotation) (Variables|Default|GetScale))))

(fn ConstructionScript)