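; Biometric door switch that toggles linked doors when the player presses E inside its trigger volume.
; Trigger overlap enables input and opens a gate, while leaving disables input.
; A locked switch shows the locked light for three seconds before resetting.
; An unlocked switch shows the unlocked light, requires a Character overlapper, and opens or closes the SelectedActors doors based on the first one's state, restoring its default material on close.
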(event OnComponentBeginOverlap(TriggerVolume)
  (params (OverlappedComponent :type Primitive%20Component%20Object%20Reference) (OtherActor :type Actor%20Object%20Reference) (OtherComp :type Primitive%20Component%20Object%20Reference) (OtherBodyIndex :type Integer) (bFromSweep :type Boolean) (SweepResult :type Hit%20Result%20Structure%20%28by%20ref%29))
  (bind _selectedactors (Variables|Public|GetSelectedActors))
  (bind _biometric_door_switch (Variables|Default|Getbiometric%20door%20switch))
  (Input|EnableInput (Game|GetPlayerController 0))
  (Utilities|FlowControl|Gate true) ; enters at Open
)

(event OnComponentEndOverlap(TriggerVolume)
  (params (OverlappedComponent :type Primitive%20Component%20Object%20Reference) (OtherActor :type Actor%20Object%20Reference) (OtherComp :type Primitive%20Component%20Object%20Reference) (OtherBodyIndex :type Integer))
  (Input|DisableInput (Game|GetPlayerController 0)))

(event Input|KeyboardEvents|E
  (params (Key :type Key%20Structure :default "AnyKey"))
  (bind _selectedactors (Variables|Public|GetSelectedActors))
  (bind _biometric_door_switch (Variables|Default|Getbiometric%20door%20switch))
  (:Pressed
    (Utilities|FlowControl|Gate true
      (:Exit
        (if (Variables|Default|GetisLocked)
          (Rendering|Material|SetMaterial (Variables|Default|Getbiometric%20door%20switch) 0 "/Game/Materials/Door_Locked_Light.Door_Locked_Light")
          (Audio|PlaySound2D "/Game/Blueprints/Door_with_switch/Unlocked.Unlocked")
          (Utilities|FlowControl|Delay 3.0)
          (Rendering|Material|SetMaterial _biometric_door_switch 0 "/Game/Materials/DoorControllerDef.DoorControllerDef")
          (else
            (Rendering|Material|SetMaterial (Variables|Default|Getbiometric%20door%20switch) 0 "/Game/Materials/Door_Unlocked_Light.Door_Unlocked_Light")
            (Audio|PlaySound2D "/Game/Blueprints/Door_with_switch/Unlocked.Unlocked")
            (Utilities|Casting|CastToCharacter (stale OnComponentBeginOverlap(TriggerVolume) OtherActor))
            (for _array_element _selectedactors
              (if (Variables|/Game/Blueprints/Door_with_switch/BasicWhiteDoor.BasicWhiteDoor_C|GetDoorOpen (Utilities|Array|Get(acopy) _selectedactors))
                (Default|CloseDoor _selectedactors)
                (Rendering|Material|SetMaterial _biometric_door_switch 0 "/Game/Materials/DoorControllerDef.DoorControllerDef")
                (else
                  (Default|OpenDoor _selectedactors))))))))))

(fn ConstructionScript)