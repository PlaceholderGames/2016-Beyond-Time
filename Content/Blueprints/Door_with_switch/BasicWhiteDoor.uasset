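; BasicWhiteDoor is a door actor that slides open and closed when its OpenDoor or CloseDoor events are called.
; The construction script caches the placed location, and each event sets a DoorOpen flag and plays a 2D sound.
; A DoorMovment timeline plays forward to open and in reverse to close, adding its vector track to that cached location without sweeping.
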(event Custom|OpenDoor
  (Variables|Public|SetDoorOpen true)
  (Utilities|FlowControl|Sequence
    (:then_0
      (Audio|PlaySound2D "/Game/Blueprints/Door_with_switch/OpenDoor.OpenDoor"))
    (:then_1
      (bind _doorlocation (Timeline|DoorMovment Play)
        (:Update
          (Transformation|SetActorLocation (+ (Variables|Default|GetInitalLocation) _doorlocation) false false))))))

(event Custom|CloseDoor
  (Variables|Public|SetDoorOpen false)
  (Utilities|FlowControl|Sequence
    (:then_0
      (Audio|PlaySound2D "/Game/Blueprints/Door_with_switch/CloseDoor.CloseDoor"))
    (:then_1
      (bind _doorlocation (Timeline|DoorMovment Reverse)
        (:Update
          (Transformation|SetActorLocation (+ (Variables|Default|GetInitalLocation) _doorlocation) false false))))))

(fn ConstructionScript
  (bind _returnvalue (Transformation|GetActorLocation))
  (Transformation|SetActorLocation _returnvalue false false)
  (Variables|Default|SetInitalLocation _returnvalue))